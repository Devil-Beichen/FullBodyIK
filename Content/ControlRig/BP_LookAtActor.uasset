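; BP_LookAtActor is a look-at target that third-person characters track while inside its sphere.
; Sphere overlap sets the character's LookAtObject to this actor and enables IsLookAt, then clears both on exit.
; On BeginPlay, a timeline lerps the mesh between StartLocation and a point 200 units along world Y.
; Tick refreshes StartLocation from the actor's location; leftover rotation and offset nodes are unconnected.
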(event `self.ReceiveBeginPlay`
  (`self.移动`))

(event `self.ReceiveTick`
  (params (DeltaSeconds :type "Float (single-precision)"))
  (set `self.StartLocation` (`self.K2_GetActorLocation`)))

(event `移动`
  (bind _startlocation (`self.StartLocation`))
  (bind (_direction _line) (`Timeline|Timeline` :!via `PlayFromStart`)
    (:`Update`
      (`SceneComponent.K2_SetWorldLocation` (`self.Mesh`) (`KismetMathLibrary.VLerp` _startlocation (+ _startlocation (0.0 200.0 0.0)) _line) false false))))

(event `self.Sphere.OnComponentBeginOverlap`
  (params (OverlappedComponent :type "PrimitiveComponent Object Reference") (OtherActor :type "Actor Object Reference") (OtherComp :type "PrimitiveComponent Object Reference") (OtherBodyIndex :type Integer) (bFromSweep :type Boolean) (SweepResult :type "HitResult Structure (by ref)"))
  (bind _asbp_third_person_character (cast `/Game/ThirdPerson/Blueprints/BP_ThirdPersonCharacter` OtherActor))
  (set `/Game/ThirdPerson/Blueprints/BP_ThirdPersonCharacter.LookAtObject` self _asbp_third_person_character)
  (set `/Game/ThirdPerson/Blueprints/BP_ThirdPersonCharacter.IsLookAt` true _asbp_third_person_character))

(event `self.Sphere.OnComponentEndOverlap`
  (params (OverlappedComponent :type "PrimitiveComponent Object Reference") (OtherActor :type "Actor Object Reference") (OtherComp :type "PrimitiveComponent Object Reference") (OtherBodyIndex :type Integer))
  (bind _asbp_third_person_character (cast `/Game/ThirdPerson/Blueprints/BP_ThirdPersonCharacter` OtherActor))
  (set `/Game/ThirdPerson/Blueprints/BP_ThirdPersonCharacter.LookAtObject` null _asbp_third_person_character)
  (set `/Game/ThirdPerson/Blueprints/BP_ThirdPersonCharacter.IsLookAt` false _asbp_third_person_character))

(fn `UserConstructionScript`)