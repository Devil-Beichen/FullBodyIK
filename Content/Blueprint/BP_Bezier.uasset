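; Actor that flies to a Target along a randomized Bezier curve over TimeL seconds, then snaps back to its start and destroys itself.
; SetStartAndEndLocation builds control points between actor and Target, randomly offsetting some sideways and vertically.
; A timeline drives GetBezierCurve, which recursively interpolates point pairs (De Casteljau) to position the actor.
; During flight, Tick draws a debug trail and updates the last point to follow the moving Target.
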(event Custom|Move
  (CallFunction|SetStartandEndLocation)
  (if (Utilities|Array|IsValidIndex (Variables|Default|GetPoints) 1)
    (Components|Timeline|SetPlayRate (Variables|Default|GetTimeLine) (/ 1.0 (Variables|Default|GetTimeL)))
    (bind _time (Timeline|TimeLine PlayFromStart)
      (:Update
        (Variables|Default|SetCanDebug true)
        (CallFunction|GetBezierCurve (Variables|Default|GetPoints) _time (Variables|Default|GetTimeL)))
      (:Finished
        (Transformation|SetActorLocation (Utilities|Array|Get(acopy) (Variables|Default|GetPoints)) false false)
        (Variables|Default|SetCanDebug false)
        (Actor|DestroyActor)))))

(event EventBeginPlay
  (CallFunction|Move)
  (bind _output_get (Variables|Default|SetLocation (Transformation|GetActorLocation)))
  (Variables|Default|SetLocationLast _output_get))

(event Collision|EventActorBeginOverlap
  (params (OtherActor :type Actor%20Object%20Reference)))

(event EventTick
  (params (DeltaSeconds :type Float%20%28single-precision%29))
  (bind _points (Variables|Default|GetPoints))
  (Variables|Default|SetLocationLast (Variables|Default|GetLocation))
  (Variables|Default|SetLocation (Transformation|GetActorLocation))
  (if (Variables|Default|GetCanDebug)
    (Rendering|Debug|DrawDebugLine (Variables|Default|GetLocationLast) (Variables|Default|GetLocation) "(R=1.000000,G=1.000000,B=0.000000,A=1.000000)" 1.0 1.0)
    (Utilities|Array|SetArrayElem _points (- (Utilities|Array|Length _points) 1) (Transformation|GetActorLocation (Variables|Default|GetTarget)) true)))

(fn ConstructionScript
  (CallFunction|SetStartandEndLocation))

(fn GetBezierCurve
  (params (Points :type Array%20of%20Vectors) (CurveTime :type Float%20%28double-precision%29) (TolalTime :type Float%20%28double-precision%29))
  (LocalVariables|SetTime (/ CurveTime TolalTime))
  (bind _output_get (LocalVariables|SetCount (Utilities|Array|Length Points)))
  (for _index (range 0 (- _output_get 2))
    (Utilities|Array|Add (LocalVariables|GetPoints_Delta) (|(Start+((End-Start)*{9C10BC15-45E2-D868-963A-FEBA7E420567})) (Utilities|Array|Get(acopy) Points _index) (Utilities|Array|Get(acopy) Points (+ _index 1)))))
  (if (== (Utilities|Array|Length (LocalVariables|GetPoints_Delta)) 1)
    (Transformation|SetActorLocation (Utilities|Array|Get(acopy) (LocalVariables|GetPoints_Delta)) false false)
    (else
      (CallFunction|GetBezierCurve (LocalVariables|GetPoints_Delta) CurveTime TolalTime))))

(fn SetStartandEndLocation
  (bind _returnvalue (Transformation|GetActorLocation))
  (bind _returnvalue_2 (Math|Random|RandomFloatinRange -1.0 1.0))
  (bind _points (Variables|Default|GetPoints))
  (bind _last_index (Variables|Default|GetLast%20Index))
  (bind _target (Variables|Default|GetTarget))
  (bind _returnvalue_3 (Transformation|GetActorLocation _target))
  (bind _returnvalue_4 (- _returnvalue_3 _returnvalue))
  (bind _returnvalue_5 (Math|Vector|VectorLength _returnvalue_4))
  (bind _returnvalue_6 (/ _returnvalue_5 _last_index))
  (bind _returnvalue_7 (* _returnvalue_6 _returnvalue_2))
  (Variables|Default|GetTarget
    (:then
      (Utilities|Array|Clear (Variables|Default|GetPoints))
      (for _index (range 0 (- _last_index 1))
        (Utilities|Array|Add (Variables|Default|GetPoints) (Math|Transform|TransformLocation (Transformation|GetActorTransform) (Math|Vector|MakeVector (* (.x (Math|Vector|GetForwardVector (Math|Rotator|MakeRotfromX _returnvalue_4))) (* _returnvalue_6 _index)) (* (Utilities|Select :Index _index :Option%200 0.0 :Option%201 _returnvalue_7 :Option%202 0.0 :Option%203 _returnvalue_7 :Option%204 0.0) 2.0) (* (Utilities|Select :Index _index :Option%200 0.0 :Option%201 _returnvalue_6 :Option%202 0.0 :Option%203 (* _returnvalue_6 1.0) :Option%204 0.0) (Math|Random|RandomFloatinRange -1.0 1.0))))))
      (Utilities|Array|SetArrayElem _points 0 (Transformation|GetActorLocation) true)
      (Utilities|Array|SetArrayElem _points (- (Utilities|Array|Length _points) 1) (Transformation|GetActorLocation (Variables|Default|GetTarget)) true))
    (:else)))