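; CBP_AutoFloor is a component that makes its owning Static Mesh Actor rock back and forth on its own, as an automatically tilting floor.
; On BeginPlay it caches the owner's static mesh component, provided the owner is a StaticMeshActor.
; Each Tick it overwrites the mesh's relative rotation with sine waves of game time, using per-axis Speed and Angles for roll and pitch, with yaw held at zero.
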(event `self.ReceiveBeginPlay`
  (bind _asstatic_mesh_actor (cast `StaticMeshActor` (`self.GetOwner`)))
  (set `self.Mesh` (`StaticMeshActor.StaticMeshComponent` _asstatic_mesh_actor)))

(event `self.ReceiveTick`
  (params (DeltaSeconds :type "Float (single-precision)"))
  (bind _returnvalue (`KismetSystemLibrary.GetGameTimeInSeconds`))
  (bind (_speed_x _speed_y) (`KismetMathLibrary.BreakVector` (`self.Speed`)))
  (bind (_angles_x _angles_y) (`KismetMathLibrary.BreakVector` (`self.Angles`)))
  (bind _mesh (`self.Mesh`)
    (:`then`
      (`SceneComponent.K2_SetRelativeRotation` _mesh (`KismetMathLibrary.MakeRotator` (* (`KismetMathLibrary.Sin` (* _speed_x _returnvalue)) _angles_x) (* (`KismetMathLibrary.Sin` (* _returnvalue _speed_y)) _angles_y)) false false))
    (:`else`)))