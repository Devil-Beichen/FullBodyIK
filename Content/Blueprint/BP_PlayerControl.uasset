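; BP_PlayerControl is a player controller that turns input into movement, look and jump on the possessed Character.
; Tick re-caches the controlled pawn as MyCharacter whenever it changes.
; Gamepad look is scaled by delta time and a fixed rate, while mouse look passes through raw.
; Move axes call MovementInput, which moves the character along forward or right vectors built only from control yaw.
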(event `self.ReceiveBeginPlay`)

(event `self.ReceiveTick`
  (params (DeltaSeconds :type "Float (single-precision)"))
  (bind _returnvalue (`self.K2_GetPawn`))
  (if (not (== (`self.MyCharacter`) _returnvalue))
    (bind _ascharacter (cast `Character` _returnvalue))
    (set `self.MyCharacter` _ascharacter)))

(event `InputAxis|Turn Right / Left Gamepad`
  (params (AxisValue :type "Float (single-precision)"))
  (bind _mycharacter (`self.MyCharacter`)
    (:`then`
      (`Pawn.AddControllerYawInput` _mycharacter (* AxisValue (`GameplayStatics.GetWorldDeltaSeconds`) 50.0)))
    (:`else`)))

(event `InputAxis|Turn Right / Left Mouse`
  (params (AxisValue :type "Float (single-precision)"))
  (bind _mycharacter (`self.MyCharacter`)
    (:`then`
      (`Pawn.AddControllerYawInput` _mycharacter AxisValue))
    (:`else`)))

(event `InputAxis|Look Up / Down Gamepad`
  (params (AxisValue :type "Float (single-precision)"))
  (bind _mycharacter (`self.MyCharacter`)
    (:`then`
      (`Pawn.AddControllerPitchInput` _mycharacter (* AxisValue (`GameplayStatics.GetWorldDeltaSeconds`) 50.0)))
    (:`else`)))

(event `InputAxis|Look Up / Down Mouse`
  (params (AxisValue :type "Float (single-precision)"))
  (bind _mycharacter (`self.MyCharacter`)
    (:`then`
      (`Pawn.AddControllerPitchInput` _mycharacter AxisValue))
    (:`else`)))

(event `InputAction|Jump`
  (params (Key :type "Key Structure"))
  (:`Pressed`
    (bind _mycharacter (`self.MyCharacter`)
      (:`then`
        (`Character.Jump` _mycharacter))
      (:`else`)))
  (:`Released`
    (`Character.StopJumping` _mycharacter)))

(event `InputAxis|Move Forward / Backward`
  (params (AxisValue :type "Float (single-precision)"))
  (`self.MyCharacter`
    (:`then`
      (`self.MovementInput` true))
    (:`else`)))

(event `InputAxis|Move Right / Left`
  (params (AxisValue :type "Float (single-precision)"))
  (`self.MyCharacter`
    (:`then`
      (`self.MovementInput` false))
    (:`else`)))

(fn `MovementInput`
  (params (`Axis F` :type Boolean :default false))
  (bind (_returnvalue_roll _returnvalue_pitch _returnvalue_yaw) (`KismetMathLibrary.BreakRotator` (`self.GetControlRotation`)))
  (bind _mycharacter (`self.MyCharacter`))
  (if `Axis F`
    (`Pawn.AddMovementInput` _mycharacter (`KismetMathLibrary.GetForwardVector` (`KismetMathLibrary.MakeRotator` 0.0 0.0 _returnvalue_yaw)) (`self.GetInputAxisValue`) false)
    (else
      (`Pawn.AddMovementInput` _mycharacter (`KismetMathLibrary.GetRightVector` (`KismetMathLibrary.MakeRotator` 0.0 0.0 _returnvalue_yaw)) (`self.GetInputAxisValue`) false))))

(fn `UserConstructionScript`)